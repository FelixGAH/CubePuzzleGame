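; Player controller for a cube-grid puzzle, handling gamepad cube selection and an inventory interface.
; BeginPlay creates the UI, switches to the puzzle camera, caches all cubes, selects the starting cube and flags its neighbors via selection-actor overlaps.
; Delayed left-stick checks move the selection by row or column, re-running the search loop to skip blocked cubes.
; A and B open and close inventory mode, where the stick moves the widget highlight.
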(event Custom|SetCamera
  ;[1 1 1] Set Camera
  (bind _outactors (Actor|GetAllActorsOfClass "/Game/GameSettings/BP_PuzzleCamera.BP_PuzzleCamera_C"))
  (Game|Player|SetViewTargetwithBlend (Utilities|Array|Get(acopy) _outactors) 0.0 "VTBlend_Linear" 0.0 false))

(event Custom|GetAllCubes
  ;[1 1 1] Save all Cubes into Array
  (bind _outactors (Actor|GetAllActorsOfClass "/Game/Cubes/BP_Cube_Master.BP_Cube_Master_C"))
  (Variables|Default|SetLevelCubes _outactors))

(event Custom|NavigateInventory
  (bind _sticky (Class|PlayerController|GetInputAnalogStickState "CAS_LeftStick"))
  (bind _interface (Variables|Default|GetInterface))
  (Utilities|FlowControl|Sequence
    (:then_0
      (Utilities|FlowControl|DoOnce true
        (:Completed
          (Default|SetSelectionHighlight _interface)
          (Default|Activate/DeactivateInterface _interface))))
    (:then_1
      (Utilities|FlowControl|Delay 0.15)
      (if (<= _sticky -0.8)
        (Default|SetSelectionHighlight (Variables|Default|GetInterface) 1)
        (elif (>= _sticky 0.8)
          (Default|SetSelectionHighlight (Variables|Default|GetInterface) -1))))))

(event Custom|ResetInterface
  (bind _interface (Variables|Default|GetInterface))
  (Utilities|FlowControl|DoOnce true) ; enters at Reset
)

(event EventBeginPlay
  (bind _returnvalue (UserInterface|CreateWidget "/Game/UserInterface/WB_PuzzleInterface.WB_PuzzleInterface_C" (Game|GetPlayerController 0)))
  (bind _output_get (Variables|Default|SetInterface _returnvalue))
  (UserInterface|Viewport|AddtoViewport _output_get 0)
  (CallFunction|GetAllCubes)
  (CallFunction|SetCamera)
  (Utilities|FlowControl|Delay 0.2)
  (bind _array_element (Utilities|Array|ForEachLoopwithBreak (Variables|Default|GetLevelCubes) :!label _label)
    (:LoopBody
      (if (Variables|/Game/Cubes/BP_Cube_Master.BP_Cube_Master_C|GetisStartingPosition _array_element)
        (goto _label Break)))
    (:Completed
      (bind _returnvalue_2 (Game|SpawnActorfromClass "/Game/Character/BP_SelectionActor.BP_SelectionActor_C" (Math|Transform|MakeTransform (Transformation|GetActorLocation _array_element) "0, 0, 0" "1,1,1") "Undefined" 0 0))
      (Variables|Default|SetSelectionActor _returnvalue_2)
      (bind _output_get_2 (Variables|Default|SetSelectedCube _array_element))
      (Default|CubeIsSelected _output_get_2)
      (CallFunction|SetStartAdjacentCubes))))

(event Input|ActionEvents|InputActionThumbstickXAxis
  (params (Key :type Key%20Structure :default "None"))
  (bind _sticky (Class|PlayerController|GetInputAnalogStickState "CAS_LeftStick"))
  (:Pressed
    (if (not (Variables|Default|GetinInventory))
      (Utilities|FlowControl|Sequence
        (:then_0
          (Utilities|FlowControl|Delay 0.15)
          (if (>= _sticky 0.8)
            (CallFunction|SetNewSelection false -1)))
        (:then_1
          (Utilities|FlowControl|Delay 0.15)
          (if (<= _sticky -0.8)
            (CallFunction|SetNewSelection false 1)))))))

(event Input|ActionEvents|InputActionThumbstickYAxis
  (params (Key :type Key%20Structure :default "None"))
  (bind _stickx (Class|PlayerController|GetInputAnalogStickState "CAS_LeftStick"))
  (:Pressed
    (if (Variables|Default|GetinInventory)
      (CallFunction|NavigateInventory)
      (else
        (Utilities|FlowControl|Sequence
          (:then_0
            (Utilities|FlowControl|Delay 0.15)
            (if (>= _stickx 0.8)
              (CallFunction|SetNewSelection true 1)))
          (:then_1
            (Utilities|FlowControl|Delay 0.15)
            (if (<= _stickx -0.8)
              (CallFunction|SetNewSelection true -1))))))))

(event Input|ActionEvents|InputActionA_Button
  (params (Key :type Key%20Structure :default "None"))
  (:Pressed
    (if (not (Variables|Default|GetinInventory))
      (Variables|Default|SetinInventory true)
      (CallFunction|ResetInterface)
      (CallFunction|NavigateInventory))))

(event Input|ActionEvents|InputActionB_Button
  (params (Key :type Key%20Structure :default "None"))
  (:Pressed
    (if (Variables|Default|GetinInventory)
      (Variables|Default|SetinInventory false)
      (Default|Activate/DeactivateInterface (Variables|Default|GetInterface)))))

(fn ConstructionScript)

(fn SetStartAdjacentCubes
  (bind _selectionactor (Variables|Default|GetSelectionActor))
  (LocalVariables|SetAdjacentCubes (Collision|GetOverlappingActors (Variables|/Game/Character/BP_SelectionActor.BP_SelectionActor_C|GetAdjacentCubesRow _selectionactor) "/Game/Cubes/BP_Cube_Master.BP_Cube_Master_C" :!class /Script/Engine.PrimitiveComponent))
  (for _array_element (Collision|GetOverlappingActors (Variables|/Game/Character/BP_SelectionActor.BP_SelectionActor_C|GetAdjacentCubesColumn _selectionactor) "/Game/Cubes/BP_Cube_Master.BP_Cube_Master_C" :!class /Script/Engine.PrimitiveComponent)
    (Utilities|Array|Add (LocalVariables|GetAdjacentCubes) _array_element))
  (Utilities|Array|RemoveItem (LocalVariables|GetAdjacentCubes) (Variables|Default|GetSelectedCube))
  (for _array_element_2 (LocalVariables|GetAdjacentCubes)
    (bind _asbp_cube_master (Utilities|Casting|CastToBP_Cube_Master _array_element_2))
    (Default|CubeIsAdjacent _asbp_cube_master)))

(fn SetNewSelection
  (params (isY :type Boolean) (+/- :type Integer))
  (if isY
    ;[1 1 1] Move along row
    (LocalVariables|SetNextIndex +/-)
    (if (or (<= (+ (Variables|/Game/Cubes/BP_Cube_Master.BP_Cube_Master_C|GetColumn (Variables|Default|GetSelectedCube)) (LocalVariables|GetNextIndex)) 6) (>= (+ (Variables|/Game/Cubes/BP_Cube_Master.BP_Cube_Master_C|GetColumn (Variables|Default|GetSelectedCube)) (LocalVariables|GetNextIndex)) 1))
      (bind _array_element (Utilities|Array|ForEachLoopwithBreak (Variables|Default|GetLevelCubes) :!label _label)
        (:LoopBody
          (if (and (== (Variables|/Game/Cubes/BP_Cube_Master.BP_Cube_Master_C|GetRow _array_element) (Variables|/Game/Cubes/BP_Cube_Master.BP_Cube_Master_C|GetRow (Variables|Default|GetSelectedCube))) (== (Variables|/Game/Cubes/BP_Cube_Master.BP_Cube_Master_C|GetColumn _array_element) (+ (Variables|/Game/Cubes/BP_Cube_Master.BP_Cube_Master_C|GetColumn (Variables|Default|GetSelectedCube)) (LocalVariables|GetNextIndex))))
            (if (Variables|/Game/Cubes/BP_Cube_Master.BP_Cube_Master_C|GetisBlocked _array_element)
              (Utilities|FlowControl|Sequence
                (:then_0
                  (if (<= (LocalVariables|GetNextIndex) -1)
                    (LocalVariables|SetNextIndex (+ (LocalVariables|GetNextIndex) -1))
                    (goto _label)))
                (:then_1
                  (if (>= (LocalVariables|GetNextIndex) 1)
                    (LocalVariables|SetNextIndex (+ (LocalVariables|GetNextIndex) 1))
                    (goto _label))))
              (else
                (Utilities|FlowControl|Sequence
                  (:then_0
                    (goto _label_2 Reset))
                  (:then_1
                    (goto _label Break)))))))
        (:Completed
          (Utilities|FlowControl|DoOnce true :!label _label_2
            (:Completed
              (Default|CubeDeselection (Variables|Default|GetSelectedCube))
              (bind _output_get (Variables|Default|SetSelectedCube _array_element))
              (Default|CubeIsSelected _output_get)
              (Transformation|SetActorLocation (Variables|Default|GetSelectionActor) (Transformation|GetActorLocation _output_get) false false))))))
    (else
      ;[1 1 1] Move along column
      (LocalVariables|SetNextIndex +/-)
      (if (and (<= (+ (Variables|/Game/Cubes/BP_Cube_Master.BP_Cube_Master_C|GetRow (Variables|Default|GetSelectedCube)) (LocalVariables|GetNextIndex)) 6) (>= (+ (Variables|/Game/Cubes/BP_Cube_Master.BP_Cube_Master_C|GetRow (Variables|Default|GetSelectedCube)) (LocalVariables|GetNextIndex)) 1))
        (bind _array_element_2 (Utilities|Array|ForEachLoopwithBreak (Variables|Default|GetLevelCubes) :!label _label_3)
          (:LoopBody
            (if (and (== (Variables|/Game/Cubes/BP_Cube_Master.BP_Cube_Master_C|GetColumn _array_element_2) (Variables|/Game/Cubes/BP_Cube_Master.BP_Cube_Master_C|GetColumn (Variables|Default|GetSelectedCube))) (== (Variables|/Game/Cubes/BP_Cube_Master.BP_Cube_Master_C|GetRow _array_element_2) (+ (Variables|/Game/Cubes/BP_Cube_Master.BP_Cube_Master_C|GetRow (Variables|Default|GetSelectedCube)) (LocalVariables|GetNextIndex))))
              (if (Variables|/Game/Cubes/BP_Cube_Master.BP_Cube_Master_C|GetisBlocked _array_element_2)
                (Utilities|FlowControl|Sequence
                  (:then_0
                    (if (<= (LocalVariables|GetNextIndex) -1)
                      (LocalVariables|SetNextIndex (+ (LocalVariables|GetNextIndex) -1))
                      (goto _label_3)))
                  (:then_1
                    (if (>= (LocalVariables|GetNextIndex) 1)
                      (LocalVariables|SetNextIndex (+ (LocalVariables|GetNextIndex) 1))
                      (goto _label_3))))
                (else
                  (Utilities|FlowControl|Sequence
                    (:then_0
                      (goto _label_4 Reset))
                    (:then_1
                      (goto _label_3 Break)))))))
          (:Completed
            (Utilities|FlowControl|DoOnce true :!label _label_4
              (:Completed
                (Default|CubeDeselection (Variables|Default|GetSelectedCube))
                (bind _output_get_2 (Variables|Default|SetSelectedCube _array_element_2))
                (Default|CubeIsSelected _output_get_2)
                (Transformation|SetActorLocation (Variables|Default|GetSelectionActor) (Transformation|GetActorLocation _output_get_2) false false)))))))))