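; BP_PathPiece_Master is a path piece, by its name the base for the others, that updates which neighbouring cubes count as adjacent.
; CheckOverlappingCubes un-marks the adjacent cubes in the passed Owner's NeighbourCubes, then refills that array with the first BP_Cube_Master overlapping each of three overlap components.
; New neighbours that are not developed get marked adjacent.
; An unconnected debug variant uses a local OverlappingCubes array instead.
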(event Custom|CheckOverlappingCubes
  (params (Owner :type BP%20Cube%20Master%20Object%20Reference))
  (bind _neighbourcubes (Variables|/Game/Cubes/BP_Cube_Master.BP_Cube_Master_C|GetNeighbourCubes Owner))
  (if (> (Utilities|Array|Length _neighbourcubes) 0)
    (for _array_element _neighbourcubes
      (bind _asbp_cube_master (Utilities|Casting|CastToBP_Cube_Master _array_element))
      (if (Variables|/Game/Cubes/BP_Cube_Master.BP_Cube_Master_C|GetisAdjacent _asbp_cube_master)
        (Default|CubeIsNotAdjacent _asbp_cube_master)))
    (Utilities|Array|Clear _neighbourcubes))
  (Utilities|Array|Add _neighbourcubes (Utilities|Array|Get(acopy) (Collision|GetOverlappingActors (Variables|Default|GetCubeOverlap01) "/Game/Cubes/BP_Cube_Master.BP_Cube_Master_C" :!class /Script/Engine.PrimitiveComponent)))
  (Utilities|Array|Add _neighbourcubes (Utilities|Array|Get(acopy) (Collision|GetOverlappingActors (Variables|Default|GetCubeOverlap02) "/Game/Cubes/BP_Cube_Master.BP_Cube_Master_C" :!class /Script/Engine.PrimitiveComponent)))
  (Utilities|Array|Add _neighbourcubes (Utilities|Array|Get(acopy) (Collision|GetOverlappingActors (Variables|Default|GetCubeOverlap03) "/Game/Cubes/BP_Cube_Master.BP_Cube_Master_C" :!class /Script/Engine.PrimitiveComponent)))
  (for _array_element_2 _neighbourcubes
    (bind _asbp_cube_master_2 (Utilities|Casting|CastToBP_Cube_Master _array_element_2))
    (if (not (Variables|/Game/Cubes/BP_Cube_Master.BP_Cube_Master_C|GetisDeveloped _asbp_cube_master_2))
      (Default|CubeIsAdjacent _asbp_cube_master_2))))

(event EventBeginPlay)

(fn ConstructionScript)