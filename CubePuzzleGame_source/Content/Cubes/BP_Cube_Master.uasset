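; BP_Cube_Master is a cube Blueprint that highlights itself according to selection, adjacency and blocked state.
; BeginPlay creates a dynamic material instance, and selection and adjacency events set flags, then run SetCubeHighlighting.
; That function sets color and intensity: bright green for selected, bright red for unblocked adjacent, dim tan otherwise.
; SetNeighbourCubes marks this cube itself adjacent when it finds an undeveloped cube in NeighbourCubes.
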(event Custom|CubeIsNotAdjacent
  (Variables|CubeStatus|SetisAdjacent false)
  (CallFunction|SetCubeHighlighting))

(event Custom|CubeIsSelected
  (Variables|CubeStatus|SetisSelected true)
  (CallFunction|SetCubeHighlighting))

(event Custom|CubeIsAdjacent
  (Variables|CubeStatus|SetisAdjacent true)
  (CallFunction|SetCubeHighlighting))

(event Custom|CubeDeselection
  (Variables|CubeStatus|SetisSelected false)
  (CallFunction|SetCubeHighlighting))

(event Custom|SetNeighbourCubes
  (for _array_element (Variables|Default|GetNeighbourCubes)
    (bind _asbp_cube_master (Utilities|Casting|CastToBP_Cube_Master _array_element))
    (if (not (Variables|BP_Cube_Master_C|GetisDeveloped _asbp_cube_master))
      (CallFunction|CubeIsAdjacent))))

(event EventBeginPlay
  (bind _returnvalue (Rendering|Material|CreateDynamicMaterialInstance (Variables|Default|GetCubeMesh) 0 "/Game/CuteSpace/Materials/Cube_01d_Mat.Cube_01d_Mat" "None" :!class /Script/Engine.PrimitiveComponent))
  (Variables|Default|SetMaterialInstance _returnvalue))

(fn ConstructionScript)

(fn SetCubeHighlighting
  (bind _materialinstance (Variables|Default|GetMaterialInstance))
  (bind _materialinstance_2 (Variables|Default|GetMaterialInstance))
  (bind _materialinstance_3 (Variables|Default|GetMaterialInstance))
  (Utilities|FlowControl|Sequence
    (:then_0
      (if (Variables|CubeStatus|GetisSelected)
        (Rendering|Material|SetVectorParameterValue _materialinstance_2 "Color" "(R=0.163822,G=1.000000,B=0.000000,A=1.000000)" :!class /Script/Engine.MaterialInstanceDynamic :!label _label)
        (Rendering|Material|SetScalarParameterValue _materialinstance_2 "Intensity" 1e+02 :!class /Script/Engine.MaterialInstanceDynamic)))
    (:then_1
      (if (Variables|CubeStatus|GetisAdjacent)
        (if (Variables|CubeStatus|GetisSelected)
          (goto _label)
          (elif (Variables|CubeStatus|GetisBlocked)
            (Rendering|Material|SetVectorParameterValue _materialinstance "Color" "(R=0.875000,G=0.582682,B=0.446615,A=1.000000)" :!class /Script/Engine.MaterialInstanceDynamic :!label _label_2)
            (Rendering|Material|SetScalarParameterValue _materialinstance "Intensity" 1.0 :!class /Script/Engine.MaterialInstanceDynamic)
            (else
              (Rendering|Material|SetVectorParameterValue _materialinstance_3 "Color" "(R=1.000000,G=0.034090,B=0.000000,A=1.000000)" :!class /Script/Engine.MaterialInstanceDynamic)
              (Rendering|Material|SetScalarParameterValue _materialinstance_3 "Intensity" 1e+02 :!class /Script/Engine.MaterialInstanceDynamic))))))
    (:then_2
      (if (and (Math|Boolean|Equal(Boolean) (Variables|CubeStatus|GetisSelected) false) (Math|Boolean|Equal(Boolean) (Variables|CubeStatus|GetisAdjacent) false))
        (goto _label_2)))))